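; BP_Bloque is a scrolling obstacle block that scores a point when the player character passes through its Cube trigger.
; Each Tick, a macro moves it along negative X at MrSpeed scaled by delta time, and it destroys itself past a fixed X limit.
; The one-shot Cube overlap increments MPoints on BP_GS and calls OnPoint.
; Hits on Muerte and MuerteTop only print debug messages once.
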(event `self.Muerte.OnComponentHit`
  (params (HitComponent :type "PrimitiveComponent Object Reference") (OtherActor :type "Actor Object Reference") (OtherComp :type "PrimitiveComponent Object Reference") (NormalImpulse :type "Vector Structure") (Hit :type "HitResult Structure (by ref)"))
  ;[1 1 1] Muerte
  (cast `/Game/Sprites/blueprints/BluePrintCharacter` OtherActor)
  (`/Engine/EditorBlueprintResources/StandardMacros.DoOnce` false
    (:`Completed`
      (`KismetSystemLibrary.PrintString` "Colision Abajo"))))

(event `self.MuerteTop.OnComponentHit`
  (params (HitComponent :type "PrimitiveComponent Object Reference") (OtherActor :type "Actor Object Reference") (OtherComp :type "PrimitiveComponent Object Reference") (NormalImpulse :type "Vector Structure") (Hit :type "HitResult Structure (by ref)"))
  ;[1 1 1] Muerte
  (cast `/Game/Sprites/blueprints/BluePrintCharacter` OtherActor)
  (`/Engine/EditorBlueprintResources/StandardMacros.DoOnce` false
    (:`Completed`
      (`KismetSystemLibrary.PrintString` "Arriba"))))

(event `self.Cube.OnComponentBeginOverlap`
  (params (OverlappedComponent :type "PrimitiveComponent Object Reference") (OtherActor :type "Actor Object Reference") (OtherComp :type "PrimitiveComponent Object Reference") (OtherBodyIndex :type Integer) (bFromSweep :type Boolean) (SweepResult :type "HitResult Structure (by ref)"))
  ;[0 1 0.2891] Points
  (cast `/Game/Sprites/blueprints/BluePrintCharacter` OtherActor)
  (`/Engine/EditorBlueprintResources/StandardMacros.DoOnce` false
    (:`Completed`
      (`KismetSystemLibrary.PrintString` "point 1+")
      (bind _asbp_gs (cast `/Game/Blueprints/BP_GS` (`GameplayStatics.GetGameState`)))
      (`/Engine/EditorBlueprintResources/StandardMacros.IncrementInt` (`/Game/Blueprints/BP_GS.mPoints` _asbp_gs)
        (:`  `
          (`/Game/Blueprints/BP_GS.OnPoint` _asbp_gs 0))))))

(event `self.ReceiveTick`
  (params (DeltaSeconds :type "Float (single-precision)"))
  (bind _returnvalue_x (`KismetMathLibrary.BreakVector` (`self.K2_GetActorLocation`)))
  ;[1 1 1] Movimiento de los bloques
  (`|ExecutionSequence`
    (:`then_0`
      (`self.NewMacro` DeltaSeconds))
    (:`then_1`
      (if (<= _returnvalue_x -130.0)
        (`self.K2_DestroyActor`)))))

(fn `UserConstructionScript`)